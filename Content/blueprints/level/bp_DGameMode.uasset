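; Game mode Blueprint that gives each joining player a client type by login order and spawns them at a matching player start.
; On PostLogin it stamps the DPlayerController with an incrementing client index, destroys any pawn it already controls and restarts the player.
; The FindPlayerStart override calls GetAllPlayerStart, then uses that client type to index the player start array, ignoring the incoming name.
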(event `self.K2_PostLogin`
  (params (NewPlayer :type "PlayerController Object Reference"))
  (bind _returnvalue (`Controller.K2_GetPawn` (`self.m_cur_controller`)))
  ;[1 1 1] when player login -- set client type
  (bind _asdplayer_controller (cast `DPlayerController` NewPlayer))
  (bind _output_get (set `self.m_cur_controller` _asdplayer_controller))
  (set `DPlayerController.m_client_type` (`self.m_client_index`) _output_get)
  (`/Engine/EditorBlueprintResources/StandardMacros.IncrementInt` (`self.m_client_index`)
    (:`  `
      (`/Engine/EditorBlueprintResources/StandardMacros.IsValid` _returnvalue
        (:`Is Valid`
          (`self.K2_DestroyActor` _returnvalue))
        (:`Is Not Valid`
          _))
      (`self.RestartPlayer` (`self.m_cur_controller`)))))

(fn `FindPlayerStart`
  (params (Player :type "Controller Object Reference") (IncomingName :type String))
  (returns (ReturnValue :type "Actor Object Reference"))
  ;[1 1 1] 设置Player 的 Start 位置
  (bind _asdplayer_controller (cast `DPlayerController` Player))
  (`self.get_all_player_start`)
  (return (`|GetArrayItem` (`self.m_player_starts`) (`DPlayerController.m_client_type` _asdplayer_controller))))

(fn `UserConstructionScript`)